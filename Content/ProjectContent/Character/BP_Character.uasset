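; Player character Blueprint that handles movement, look and control of two carried weapons, one in hand and one on the back.
; BeginPlay caches both BP_Weapon instances from child actor components, and Enhanced Input forwards fire, reload, fire mode and laser actions to the hand weapon.
; Main and sub swap inputs check the held weapon's type, then SwapWeapon, unless it is busy, reattaches both weapons to opposite components and exchanges their references.
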(event Input|EnhancedActionEvents|EnhancedInputActionIA_Move
  (params (ActionValue :type Vector%202D%20Structure) (ElapsedSeconds :type Float%20%28double-precision%29) (TriggeredSeconds :type Float%20%28double-precision%29) (InputAction :type Input%20Action%20Object%20Reference :default "/Game/ProjectContent/Input/IA_Move.IA_Move"))
  (bind (_x _y) (Math|Vector2D|BreakVector2D ActionValue))
  (bind _returnvalue (Transformation|GetActorRotation))
  ;[0.15 0.15 0.15 0.5] Move
  (Pawn|Input|AddMovementInput (Math|Vector|GetForwardVector _returnvalue) _x false)
  (Pawn|Input|AddMovementInput (Math|Vector|GetRightVector _returnvalue) _y false))

(event Input|EnhancedActionEvents|EnhancedInputActionIA_Look
  (params (ActionValue :type Vector%202D%20Structure) (ElapsedSeconds :type Float%20%28double-precision%29) (TriggeredSeconds :type Float%20%28double-precision%29) (InputAction :type Input%20Action%20Object%20Reference :default "/Game/ProjectContent/Input/IA_Look.IA_Look"))
  (bind (_x _y) (Math|Vector2D|BreakVector2D ActionValue))
  ;[0.15 0.15 0.15 0.5] Look
  (Pawn|Input|AddControllerPitchInput _y)
  (Pawn|Input|AddControllerYawInput _x))

(event Input|EnhancedActionEvents|EnhancedInputActionIA_Fire
  (params (ActionValue :type Boolean) (ElapsedSeconds :type Float%20%28double-precision%29) (TriggeredSeconds :type Float%20%28double-precision%29) (InputAction :type Input%20Action%20Object%20Reference :default "/Game/ProjectContent/Input/IA_Fire.IA_Fire"))
  (bind _handweapon (Variables|Default|GetHandWeapon))
  ;[0.15 0.15 0.15 0.5] Fire
  (if ActionValue
    (Default|FirePressed _handweapon)
    (else
      (Default|FireReleased _handweapon))))

(event Input|EnhancedActionEvents|EnhancedInputActionIA_Reload
  (params (ActionValue :type Boolean) (ElapsedSeconds :type Float%20%28double-precision%29) (TriggeredSeconds :type Float%20%28double-precision%29) (InputAction :type Input%20Action%20Object%20Reference :default "/Game/ProjectContent/Input/IA_Reload.IA_Reload"))
  (bind _handweapon (Variables|Default|GetHandWeapon))
  ;[0.15 0.15 0.15 0.5] Reload
  (if (Default|CanReload _handweapon)
    (Default|Reload _handweapon)))

(event Input|EnhancedActionEvents|EnhancedInputActionIA_SwapMain
  (params (ActionValue :type Boolean) (ElapsedSeconds :type Float%20%28double-precision%29) (TriggeredSeconds :type Float%20%28double-precision%29) (InputAction :type Input%20Action%20Object%20Reference :default "/Game/ProjectContent/Input/IA_SwapMain.IA_SwapMain"))
  ;[0.15 0.15 0.15 0.5] Swap
  (switch Utilities|FlowControl|Switch|SwitchonBP_EWeaponType (Default|GetWeaponType (Variables|Default|GetHandWeapon))
    (:NewEnumerator1
      (CallFunction|SwapWeapon))))

(event Input|EnhancedActionEvents|EnhancedInputActionIA_SwapSub
  (params (ActionValue :type Boolean) (ElapsedSeconds :type Float%20%28double-precision%29) (TriggeredSeconds :type Float%20%28double-precision%29) (InputAction :type Input%20Action%20Object%20Reference :default "/Game/ProjectContent/Input/IA_SwapSub.IA_SwapSub"))
  ;[0.15 0.15 0.15 0.5] Swap
  (switch Utilities|FlowControl|Switch|SwitchonBP_EWeaponType (Default|GetWeaponType (Variables|Default|GetHandWeapon))
    (:NewEnumerator0
      (CallFunction|SwapWeapon))))

(event Input|EnhancedActionEvents|EnhancedInputActionIA_FireMode
  (params (ActionValue :type Boolean) (ElapsedSeconds :type Float%20%28double-precision%29) (TriggeredSeconds :type Float%20%28double-precision%29) (InputAction :type Input%20Action%20Object%20Reference :default "/Game/ProjectContent/Input/IA_FireMode.IA_FireMode"))
  ;[0.15 0.15 0.15 0.5] Change Fire Mode
  (Default|ChangeFireMode (Variables|Default|GetHandWeapon)))

(event Input|EnhancedActionEvents|EnhancedInputActionIA_ToggleLaserPointer
  (params (ActionValue :type Boolean) (ElapsedSeconds :type Float%20%28double-precision%29) (TriggeredSeconds :type Float%20%28double-precision%29) (InputAction :type Input%20Action%20Object%20Reference :default "/Game/ProjectContent/Input/IA_ToggleLaserPointer.IA_ToggleLaserPointer"))
  ;[0.15 0.15 0.15 0.5] ToggleLaser
  (Default|ToggleLaser (Variables|Default|GetHandWeapon)))

(event EventBeginPlay
  ;[0.15 0.15 0.15 0.5] Initialize
  (bind _asbp_weapon (Utilities|Casting|CastToBP_Weapon (Variables|/Script/Engine.ChildActorComponent|GetChildActor (Variables|Default|GetWeaponInHand))))
  (Variables|Default|SetHandWeapon _asbp_weapon)
  (bind _asbp_weapon_2 (Utilities|Casting|CastToBP_Weapon (Variables|/Script/Engine.ChildActorComponent|GetChildActor (Variables|Default|GetWeaponInBack))))
  (Variables|Default|SetBackWeapon _asbp_weapon_2))

(event Collision|EventActorBeginOverlap
  (params (OtherActor :type Actor%20Object%20Reference)))

(fn ConstructionScript)

(fn SwapWeapon
  (if (not (Default|IsBusy (Variables|Default|GetHandWeapon)))
    (LocalVariables|SetDrawWeapon (Variables|Default|GetBackWeapon))
    (LocalVariables|SetPutWeapon (Variables|Default|GetHandWeapon))
    (Transformation|AttachComponentToComponent (LocalVariables|GetDrawWeapon) (Variables|Default|GetWeaponInHand) "None" "KeepRelative" "KeepRelative" "KeepRelative" true)
    (Transformation|AttachComponentToComponent (LocalVariables|GetPutWeapon) (Variables|Default|GetWeaponInBack) "None" "KeepRelative" "KeepRelative" "KeepRelative" true)
    (Variables|Default|SetHandWeapon (LocalVariables|GetDrawWeapon))
    (Variables|Default|SetBackWeapon (LocalVariables|GetPutWeapon))))

(fn GetWeaponinHand
  (return (Variables|Default|GetHandWeapon)))