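; BP_Target is a shooting target that stands up, gets knocked down and awards score.
; Optional trigger volumes, overlapped by BP_Character, stand it up, knock it down or re-arm it to Ready.
; BP_Bullet hits on the board deplete Durability, then call KnockDown, which adds score.
; A state enum guards each transition, while Tick pitches the actor 90 degrees over a set time before settling the state.
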(event OnActorBeginOverlap(StandUpTriggerVolume)
  (params (OverlappedActor :type Actor%20Object%20Reference) (OtherActor :type Actor%20Object%20Reference)))

(event OnActorBeginOverlap(KnockDownTriggerVolume)
  (params (OverlappedActor :type Actor%20Object%20Reference) (OtherActor :type Actor%20Object%20Reference)))

(event OnActorBeginOverlap(ResetTriggerVolume)
  (params (OverlappedActor :type Actor%20Object%20Reference) (OtherActor :type Actor%20Object%20Reference)))

(event OnComponentHit(TargetBoard)
  (params (HitComponent :type Primitive%20Component%20Object%20Reference) (OtherActor :type Actor%20Object%20Reference) (OtherComp :type Primitive%20Component%20Object%20Reference) (NormalImpulse :type Vector :default "0, 0, 0") (Hit :type Hit%20Result%20Structure%20%28by%20ref%29))
  (Utilities|Casting|CastToBP_Bullet OtherActor)
  (bind _result (Math|Integer|DecrementInt (Variables|Default|GetDurability))
    (:%20%20
      (if (<= _result 0)
        (CallFunction|KnockDown)))))

(event Custom|StandUpVolumeOverlap
  (params (OverlappedActor :type Actor%20Object%20Reference) (OtherActor :type Actor%20Object%20Reference))
  (Utilities|Casting|CastToBP_Character OtherActor)
  (CallFunction|StandUp))

(event Custom|ResetVolumeOverlap
  (params (OverlappedActor :type Actor%20Object%20Reference) (OtherActor :type Actor%20Object%20Reference))
  (Utilities|Casting|CastToBP_Character OtherActor)
  (if (Utilities|Enum|Equal(Enum) (Variables|Default|GetCurrentState) "NewEnumerator2")
    (Variables|Default|SetCurrentState "NewEnumerator0")))

(event Custom|KnockDownVolumeOverlap
  (params (OverlappedActor :type Actor%20Object%20Reference) (OtherActor :type Actor%20Object%20Reference))
  (Utilities|Casting|CastToBP_Character OtherActor)
  (CallFunction|KnockDown))

(event EventBeginPlay
  (bind _standuptriggervolume (Variables|Volume|GetStandUpTriggerVolume))
  (bind _resettriggervolume (Variables|Volume|GetResetTriggerVolume))
  (bind _knockdowntriggervolume (Variables|Volume|GetKnockDownTriggerVolume))
  (Utilities|FlowControl|Sequence
    (:then_0
      (Utilities|IsValid _standuptriggervolume
        (:Is%20Valid
          (Collision|BindEventtoOnActorBeginOverlap _standuptriggervolume (delegate Custom|StandUpVolumeOverlap)))))
    (:then_1
      (Utilities|IsValid _knockdowntriggervolume
        (:Is%20Valid
          (Collision|BindEventtoOnActorBeginOverlap _knockdowntriggervolume (delegate Custom|KnockDownVolumeOverlap)))))
    (:then_2
      (Utilities|IsValid _resettriggervolume
        (:Is%20Valid
          (Collision|BindEventtoOnActorBeginOverlap _resettriggervolume (delegate Custom|ResetVolumeOverlap)))))))

(event Collision|EventActorBeginOverlap
  (params (OtherActor :type Actor%20Object%20Reference)))

(event EventTick
  (params (DeltaSeconds :type Float%20%28single-precision%29))
  (CallFunction|TickRotate DeltaSeconds))

(fn ConstructionScript)

(fn StandUp
  (if (Utilities|Enum|Equal(Enum) (Variables|Default|GetCurrentState) "NewEnumerator0")
    (Utilities|FlowControl|Sequence
      (:then_0
        (Variables|Rotation|SetRotationDegree -9e+01)
        (bind _output_get (Variables|Rotation|SetRotationTime (Variables|Rotation|GetRotaionTimeStandUp)))
        (Variables|Rotation|SetRotationRemainTime _output_get))
      (:then_1
        (Variables|Default|SetCurrentState "NewEnumerator4"))
      (:then_2
        (Audio|PlaySoundatLocation (Variables|Default|GetStandUpSound) (Transformation|GetWorldLocation (Variables|Default|GetTargetBoard)) "0, 0, 0" 1.0 1.0 0.0 0 0 0 0)))))

(fn KnockDown
  (if (Utilities|Enum|Equal(Enum) (Variables|Default|GetCurrentState) "NewEnumerator1")
    (Utilities|FlowControl|Sequence
      (:then_0
        (Variables|Rotation|SetRotationDegree 9e+01)
        (bind _output_get (Variables|Rotation|SetRotationTime (Variables|Rotation|GetRotationTimeKnockDown)))
        (Variables|Rotation|SetRotationRemainTime _output_get))
      (:then_1
        (Variables|Default|SetCurrentState "NewEnumerator3"))
      (:then_2
        (CallFunction|AddScore (Variables|Default|GetScore)))
      (:then_3
        (Audio|PlaySoundatLocation (Variables|Default|GetKnockDownSound) (Transformation|GetWorldLocation (Variables|Default|GetTargetBoard)) "0, 0, 0" 1.0 1.0 0.0 0 0 0 0)))))

(fn TickRotate
  (params (DeltaTime :type Float%20%28double-precision%29))
  (if (> (Variables|Rotation|GetRotationRemainTime) 0.0)
    (Transformation|AddActorLocalRotation (Math|Rotator|MakeRotator 0.0 (* (Math|Float|Min(Float) (Variables|Rotation|GetRotationRemainTime) DeltaTime) (/ (Variables|Rotation|GetRotationDegree) (Variables|Rotation|GetRotationTime))) 0.0) false false)
    (bind _output_get (Variables|Rotation|SetRotationRemainTime (- (Variables|Rotation|GetRotationRemainTime) DeltaTime)))
    (if (<= _output_get 0.0)
      (switch Utilities|FlowControl|Switch|SwitchonETargetState (Variables|Default|GetCurrentState)
        (:NewEnumerator4
          (Variables|Default|SetCurrentState "NewEnumerator1"))
        (:NewEnumerator3
          (Variables|Default|SetCurrentState "NewEnumerator2"))))))