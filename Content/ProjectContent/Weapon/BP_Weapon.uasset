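; BP_Weapon is a firearm actor for the player's character, with ammo, semi/full-auto modes, a toggleable laser pointer and state getters.
; Fire spawns BP_Bullet at the muzzle and, in full auto, re-schedules itself by timer until release clears it.
; Reload and draw play montages on player 0's BP_Character.
; Separate functions refill ammo and toggle the Magazine component, which stands in for the gun mesh's hidden magazine bone.
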(event EventBeginPlay
  (Components|SkinnedMesh|HideBonebyName (Variables|Default|GetGun) "b_gun_mag" "PBO_None"))

(event Collision|EventActorBeginOverlap
  (params (OtherActor :type Actor%20Object%20Reference)))

(event EventTick
  (params (DeltaSeconds :type Float%20%28single-precision%29)))

(fn ConstructionScript)

(fn Fire
  (if (> (Variables|Fire|GetRemainBullet) 0)
    (Math|Integer|DecrementInt (Variables|Fire|GetRemainBullet)
      (:%20%20
        (Utilities|FlowControl|Sequence
          (:then_0
            (bind _returnvalue (Game|SpawnActorfromClass "/Game/ProjectContent/Weapon/BP_Bullet.BP_Bullet_C" (Transformation|GetWorldTransform (Variables|Default|GetMuzzle)) "Undefined" "MultiplyWithRoot" 0 0))
            (Default|SetSpeed _returnvalue 1e+04))
          (:then_1
            (switch Utilities|FlowControl|Switch|SwitchonBP_EFireMode (Variables|Fire|GetFireMode)
              (:NewEnumerator0
                (bind _returnvalue_2 (Utilities|Time|SetTimerbyFunctionName 0 "Fire" (Variables|Fire|GetFIreInterval)))
                (Variables|Default|SetTimerHandle _returnvalue_2))))
          (:then_2
            (Audio|PlaySoundatLocation (Variables|Default|GetFireSound) (Transformation|GetWorldLocation (Variables|Default|GetMuzzle)) "0, 0, 0" 1.0 1.0 0.0 0 0 0 0)))))
    (else
      (Audio|PlaySoundatLocation (Variables|Default|GetDryFireSound) (Transformation|GetWorldLocation (Variables|Default|GetGun)) "0, 0, 0" 1.0 1.0 0.0 0 0 0 0))))

(fn GetWeaponType
  (return (Variables|Default|GetWeaponType)))

(fn ReloadStart
  (if (< (Variables|Fire|GetRemainBullet) (Variables|Fire|GetMaxBullet))
    (bind _asbp_character (Utilities|Casting|CastToBP_Character (Game|GetPlayerCharacter 0)))
    (Default|PlayMontage _asbp_character (Variables|Default|GetReloadAnimation))))

(fn IsFiring
  (return (and (Utilities|Time|IsTimerActivebyHandle (Variables|Default|GetTimerHandle)) (Variables|Fire|GetIsFirePressed))))

(fn FireReleased
  (Utilities|Time|ClearandInvalidateTimerbyHandle (Variables|Default|GetTimerHandle))
  (Variables|Fire|SetIsFirePressed false))

(fn ChangeFireMode
  (Audio|PlaySoundatLocation (Variables|Default|GetFireModeSound) (Transformation|GetWorldLocation (Variables|Default|GetGun)) "0, 0, 0" 1.0 1.0 0.0 0 0 0 0)
  (switch Utilities|FlowControl|Switch|SwitchonBP_EFireMode (Variables|Fire|GetFireMode)
    (:NewEnumerator0
      (Variables|Fire|SetFireMode "NewEnumerator1"))
    (:NewEnumerator1
      (Variables|Fire|SetFireMode "NewEnumerator0"))))

(fn GetFireMode
  (return (Variables|Fire|GetFireMode)))

(fn FirePressed
  (Variables|Fire|SetIsFirePressed true)
  (Fire|Fire))

(fn IsBusy
  (return (Fire|IsFiring)))

(fn GetWeaponName
  (return (Variables|Default|GetWeaponName)))

(fn GetRemainBullet
  (return (Variables|Fire|GetRemainBullet)))

(fn GetMaxBullet
  (return (Variables|Fire|GetMaxBullet)))

(fn CanReload
  (return (< (Variables|Fire|GetRemainBullet) (Variables|Fire|GetMaxBullet))))

(fn ToggleLaser
  (bind _asbp_laser_pointer (Utilities|Casting|CastToBP_LaserPointer (Variables|/Script/Engine.ChildActorComponent|GetChildActor (Variables|Default|GetLaserPointer))))
  (Default|ToggleLaser _asbp_laser_pointer))

(fn GetHandTransform
  (return (Variables|Default|GetHandTransform)))

(fn DoesSupportAim
  (return (Variables|Default|GetSupportAim)))

(fn ReloadComplete
  (Variables|Fire|SetRemainBullet (Variables|Fire|GetMaxBullet))
  (Audio|PlaySoundatLocation (Variables|Default|GetReloadCompleteSound) (Transformation|GetWorldLocation (Variables|Default|GetGun)) "0, 0, 0" 1.0 1.0 0.0 0 0 0 0))

(fn MagazineDetached
  (Rendering|SetVisibility (Variables|Default|GetMagazine) false false)
  (Audio|PlaySoundatLocation (Variables|Default|GetDetachMagazineSound) (Transformation|GetWorldLocation (Variables|Default|GetMagazine)) "0, 0, 0" 1.0 1.0 0.0 0 0 0 0))

(fn MagazineAttached
  (Rendering|SetVisibility (Variables|Default|GetMagazine) true false)
  (Audio|PlaySoundatLocation (Variables|Default|GetAttachMagazineSound) (Transformation|GetWorldLocation (Variables|Default|GetMagazine)) "0, 0, 0" 1.0 1.0 0.0 0 0 0 0))

(fn DrawWeapon
  (bind _asbp_character (Utilities|Casting|CastToBP_Character (Game|GetPlayerCharacter 0)))
  (Default|PlayMontage _asbp_character (Variables|Default|GetDrawAnimation)))