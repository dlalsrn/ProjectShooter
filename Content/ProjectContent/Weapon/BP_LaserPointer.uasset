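; BP_LaserPointer is a toggleable weapon laser pointer whose beam stops at the first surface it hits.
; ToggleLaser plays a sound and switches the Laser component's visibility and active state.
; While active, each Tick line-traces forward from Muzzle on the Visibility channel, storing hit distance or a fixed maximum range.
; The beam's Z scale is set from that stored distance every Tick, even while off.
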(event EventBeginPlay)

(event Collision|EventActorBeginOverlap
  (params (OtherActor :type Actor%20Object%20Reference)))

(event EventTick
  (params (DeltaSeconds :type Float%20%28single-precision%29))
  (CallFunction|TickLaser))

(fn ConstructionScript)

(fn ToggleLaser
  (Audio|PlaySoundatLocation (Variables|Default|GetToggleLaserSound) (Transformation|GetWorldLocation (Variables|Default|GetLaserPointer)) "0, 0, 0" 1.0 1.0 0.0 0 0 0 0)
  (if (Variables|Default|GetIsActivated)
    (CallFunction|TurnOff)
    (else
      (CallFunction|Turnon))))

(fn Turnon
  (Variables|Default|SetIsActivated true)
  (Rendering|SetVisibility (Variables|Default|GetLaser) true false))

(fn TurnOff
  (Variables|Default|SetIsActivated false)
  (Rendering|SetVisibility (Variables|Default|GetLaser) false false))

(fn TickLaser
  (bind _muzzle (Variables|Default|GetMuzzle))
  (bind _laser (Variables|Default|GetLaser))
  (bind _returnvalue (Transformation|GetWorldScale _laser))
  (bind _returnvalue_2 (Transformation|GetWorldLocation _muzzle))
  (bind (_x _y) (Math|Vector|BreakVector _returnvalue))
  (Utilities|FlowControl|Sequence
    (:then_0
      (if (Variables|Default|GetIsActivated)
        (bind (_outhit _returnvalue_3) (Collision|LineTraceByChannel _returnvalue_2 (+ _returnvalue_2 (* (Math|Vector|GetForwardVector _muzzle) 2.5e+03)) "TraceTypeQuery1" false 0 "None"))
        (if _returnvalue_3
          (LocalVariables|Setdistance (.Distance (Collision|BreakHitResult _outhit)))
          (else
            (LocalVariables|Setdistance 2.5e+03)))))
    (:then_1
      (Transformation|SetWorldScale3D _laser (Math|Vector|MakeVector _x _y (/ (LocalVariables|Getdistance) 1e+02))))))