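; BP_Bullet is a projectile actor that flies in a straight line and destroys itself on hit, with no damage logic in these graphs.
; Each Tick, CalculateMoveVector scales the Bullet component's forward vector by Speed and delta time, and the actor moves by that offset with a swept SetActorLocation.
; SetSpeed sets the Speed variable, and the Bullet component's hit event destroys the actor.
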(event OnComponentHit(Bullet)
  (params (HitComponent :type Primitive%20Component%20Object%20Reference) (OtherActor :type Actor%20Object%20Reference) (OtherComp :type Primitive%20Component%20Object%20Reference) (NormalImpulse :type Vector :default "0, 0, 0") (Hit :type Hit%20Result%20Structure%20%28by%20ref%29))
  (Actor|DestroyActor))

(event EventBeginPlay)

(event Collision|EventActorBeginOverlap
  (params (OtherActor :type Actor%20Object%20Reference)))

(event EventTick
  (params (DeltaSeconds :type Float%20%28single-precision%29))
  (Transformation|SetActorLocation (+ (CallFunction|CalculateMoveVector DeltaSeconds) (Transformation|GetActorLocation)) true false))

(fn ConstructionScript)

(fn CalculateMoveVector
  (params (DeltaTime :type Float%20%28double-precision%29))
  (bind _output_get (LocalVariables|SetDeltaSpeed (* DeltaTime (Variables|Default|GetSpeed))))
  (return (* _output_get (Math|Vector|GetForwardVector (Variables|Default|GetBullet)))))

(fn SetSpeed
  (params (Speed :type Float%20%28double-precision%29))
  (Variables|Default|SetSpeed Speed))