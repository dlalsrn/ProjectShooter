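; Game mode that tracks match state, score and a persistent top-ten ranking.
; StartGame and EndGame move the state from Ready through Running to End, timing the run to award a bonus for finishing under two minutes.
; Only with a positive bonus does EndGame insert the score and end timestamp into sorted parallel arrays, save, and call OnEndGame.
; Rankings load on BeginPlay from a BP_SaveGame slot.
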(event EventBeginPlay
  (CallFunction|LoadRanking))

(event EventTick
  (params (DeltaSeconds :type Float%20%28single-precision%29)))

(fn ConstructionScript)

(fn StartGame
  (switch Utilities|FlowControl|Switch|SwitchonBP_EGameState (Variables|Default|GetCurrentGameState)
    (:NewEnumerator0
      (Variables|Default|SetCurrentGameState "NewEnumerator1")
      (Variables|Default|SetStartTime (Math|DateTime|Now)))))

(fn EndGame
  (switch Utilities|FlowControl|Switch|SwitchonBP_EGameState (Variables|Default|GetCurrentGameState)
    (:NewEnumerator1
      (Variables|Default|SetCurrentGameState "NewEnumerator2")
      (Variables|Default|SetEndTime (Math|DateTime|Now))
      (bind _output_get (Variables|Default|SetElapsedTime (/ (CallFunction|GetMillisecondsfromDateTime (Variables|Default|GetEndTime) (Variables|Default|GetStartTime)) 1e+03)))
      (bind _output_get_2 (LocalVariables|SetTimeBonus (- 1.2e+02 _output_get)))
      (if (> _output_get_2 0.0)
        (CallFunction|AddScore (LocalVariables|GetTimeBonus))
        (CallFunction|UpdateRanking)
        (CallFunction|SaveRanking)
        (Default|CallOnEndGame)))))

(fn AddScore
  (params (Value :type Float%20%28double-precision%29))
  (Variables|Default|SetScore (+ Value (Variables|Default|GetScore))))

(fn GetStartTime
  (return (Variables|Default|GetStartTime)))

(fn GetGameState
  (return (Variables|Default|GetCurrentGameState)))

(fn GetScore
  (return (Variables|Default|GetScore)))

(fn LoadRanking
  (bind _returnvalue (SaveGame|LoadGamefromSlot "Ranking"))
  (bind _asbp_save_game (Utilities|Casting|CastToBP_SaveGame _returnvalue))
  (Variables|Default|SetRankingScores (Variables|/Game/ProjectContent/GamePlay/BP_SaveGame.BP_SaveGame_C|GetScores _asbp_save_game))
  (Variables|Default|SetRankingTimes (Variables|/Game/ProjectContent/GamePlay/BP_SaveGame.BP_SaveGame_C|GetTimes _asbp_save_game)))

(fn SaveRanking
  (bind _returnvalue (SaveGame|CreateSaveGameObject "/Game/ProjectContent/GamePlay/BP_SaveGame.BP_SaveGame_C"))
  (Variables|/Game/ProjectContent/GamePlay/BP_SaveGame.BP_SaveGame_C|SetScores _returnvalue (Variables|Default|GetRankingScores))
  (Variables|/Game/ProjectContent/GamePlay/BP_SaveGame.BP_SaveGame_C|SetTimes _returnvalue (Variables|Default|GetRankingTimes))
  (SaveGame|SaveGametoSlot _returnvalue "Ranking"))

(fn UpdateRanking
  (bind _rankingscores (Variables|Default|GetRankingScores))
  (bind _rankingtimes (Variables|Default|GetRankingTimes))
  (bind _endtime (Variables|Default|GetEndTime))
  (LocalVariables|SetRankingIndex 0)
  (bind _array_element (Utilities|Array|ForEachLoopwithBreak (Variables|Default|GetRankingScores) :!label _label)
    (:LoopBody
      (if (>= _array_element (Variables|Default|GetScore))
        (Math|Integer|IncrementInt (LocalVariables|GetRankingIndex))
        (else
          (goto _label Break))))
    (:Completed
      (Variables|Default|SetRanking (+ (LocalVariables|GetRankingIndex) 1))
      (Utilities|Array|Insert (Variables|Default|GetRankingScores) (Variables|Default|GetScore) (LocalVariables|GetRankingIndex))
      (Utilities|Array|Insert (Variables|Default|GetRankingTimes) (Utilities|String|Append (Utilities|String|ToString(Integer) (Class|KismetMathLibrary|GetYear _endtime)) ":" (Utilities|String|ToString(Integer) (Class|KismetMathLibrary|GetMonth _endtime)) ":" (Utilities|String|ToString(Integer) (Class|KismetMathLibrary|GetDay _endtime)) ":" (Utilities|String|ToString(Integer) (Class|KismetMathLibrary|GetHour _endtime)) ":" (Utilities|String|ToString(Integer) (Class|KismetMathLibrary|GetMinute _endtime)) ":" (Utilities|String|ToString(Integer) (Class|KismetMathLibrary|GetSecond _endtime))) (LocalVariables|GetRankingIndex))
      (if (> (Utilities|Array|Length (Variables|Default|GetRankingScores)) 10)
        (Utilities|Array|RemoveIndex _rankingscores (Utilities|Array|LastIndex _rankingscores))
        (Utilities|Array|RemoveIndex _rankingtimes (Utilities|Array|LastIndex _rankingtimes))))))

(fn GetRanking
  (return (Variables|Default|GetRanking)))

(fn GetRankingTimes
  (return (Variables|Default|GetRankingTimes)))

(fn GetRankingScores
  (return (Variables|Default|GetRankingScores)))